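; Player-controlled boot that orbits a fixed point at a radius set by its starting position, winding up and swinging like a kick.
; Tick moves it around the circle from held A/D keys and yaws it toward the center.
; Holding left mouse lowers CurrentCharge, used as pitch, to wind back; releasing raises it faster to swing forward up to a limit.
; Motion uses fixed per-frame steps, not delta time.
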(event EventBeginPlay
  (Variables|Default|SetBoot_Position (Transformation|GetActorLocation))
  (Variables|Default|SetBoot_Rotation (Transformation|GetActorRotation))
  (Variables|Default|SetAngle (Math|Trig|GetPI))
  (bind _output_get (Variables|Default|SetRadius (Math|Vector|VectorLength (- (Transformation|GetActorLocation) (Math|Vector|MakeVector 0.0 0.0 4e+02)))))
  (Development|PrintString (Utilities|String|ToString(Float) _output_get))
  (Variables|Default|SetmaxCharge 1e+02)
  (Variables|Default|SetcurrentCharge 0.0)
  (Variables|Default|SetReleaseSpeed 2.5)
  (Variables|Default|SetLaunchReady false))

(event EventTick
  (params (DeltaSeconds :type Float%20%28single-precision%29))
  (bind _returnvalue (Transformation|GetActorRotation))
  (bind (_roll _pitch _yaw) (Math|Rotator|BreakRotator _returnvalue))
  (if (Variables|Default|GetA_Pressed)
    (Variables|Default|SetAngle (- (Variables|Default|GetAngle) 0.03)))
  (if (Variables|Default|GetD_Pressed)
    (Variables|Default|SetAngle (+ (Variables|Default|GetAngle) 0.03)))
  (bind _output_get (Variables|Default|SetBoot_Position (+ (Math|Vector|MakeVector (* (Math|Trig|Cos(Radians) (Variables|Default|GetAngle)) (Variables|Default|GetRadius)) (* (Math|Trig|Sin(Radians) (Variables|Default|GetAngle)) (Variables|Default|GetRadius)) 0.0) (Math|Vector|MakeVector 0.0 0.0 4e+02))))
  (Transformation|SetActorLocation _output_get false false)
  (Transformation|SetActorRotation (Math|Rotator|MakeRotator (.Roll (Math|Rotator|BreakRotator (Math|Rotator|FindLookatRotation _output_get (Math|Vector|MakeVector 0.0 0.0 4e+02)))) (Variables|Default|GetcurrentCharge) (.Yaw (Math|Rotator|BreakRotator (Math|Rotator|FindLookatRotation _output_get (Math|Vector|MakeVector 0.0 0.0 4e+02))))))
  (if (and (Variables|Default|GetLMB_Pressed) (<= (Variables|Default|GetcurrentCharge) (Variables|Default|GetmaxCharge)))
    (if (>= (Variables|Default|GetcurrentCharge) (Math|Float|MakeLiteralFloat -9e+01))
      (Variables|Default|SetcurrentCharge (- (Variables|Default|GetcurrentCharge) 0.3))
      (Transformation|SetActorRotation (Math|Rotator|MakeRotator _roll (Variables|Default|GetcurrentCharge) _yaw) :!label _label)
      (Variables|Default|SetPrevPos (Transformation|GetActorLocation)))
    (elif (and (Variables|Default|GetLaunchReady) (<= (Variables|Default|GetcurrentCharge) (Math|Float|MakeLiteralFloat 6e+01)))
      (Variables|Default|SetcurrentCharge (+ (Variables|Default|GetcurrentCharge) (Variables|Default|GetReleaseSpeed)))
      (goto _label))))

(event Input|MouseEvents|LeftMouseButton
  (params (Key :type Key%20Structure))
  (:Pressed
    (Variables|Default|SetLMB_Pressed true)
    (Variables|Default|SetLaunchReady true))
  (:Released
    (Variables|Default|SetLMB_Pressed false)))

(event Input|KeyboardEvents|D
  (params (Key :type Key%20Structure))
  (:Pressed
    (Variables|Default|SetD_Pressed true))
  (:Released
    (Variables|Default|SetD_Pressed false)))

(event Input|KeyboardEvents|A
  (params (Key :type Key%20Structure))
  (:Pressed
    (Variables|Default|SetA_Pressed true))
  (:Released
    (Variables|Default|SetA_Pressed false)))

(fn ConstructionScript)